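; Base pickup actor that plays sounds on spawn, ground impact and destruction (consumed), with an animated spawn-in.
; A BeginPlay timeline drives scale and triggers the one-shot impact sound when elevation dips below zero, then starts sinusoidal movement and rotation.
; Tick applies the calculated location and rotation each frame.
; SetCalculatedLocation offsets height by SpawnApex, but the timeline passes it a constant zero instead of Elevation.
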(event EventBeginPlay
  (Audio|PlaySoundatLocation (Variables|Default|GetSpawnSound) (Transformation|GetActorLocation) "0, 0, 0" 1.0 1.0 0.0 0 0 0 0)
  (bind (_direction _elevation _scale) (Timeline|PickupElevationTimeline Play)
    (:Update
      (Variables|Default|SetElevation _elevation)
      (Variables|Default|SetScale _scale)
      (CallFunction|SetCalculatedLocation 0.0)
      (Transformation|SetActorScale3D (Math|Vector|MakeVector (Variables|Default|GetScale) (Variables|Default|GetScale) (Variables|Default|GetScale)))
      (if (< (Variables|Default|GetElevation) -0.1)
        (Utilities|FlowControl|DoOnce false
          (:Completed
            (Audio|PlaySoundatLocation (Variables|Default|GetGroundImpactSound) (Transformation|GetActorLocation) "0, 0, 0" 1.0 1.0 0.0 0 0 0 0)))))
    (:Finished
      (Class|AuraEffectActor|StartSinusoidalMovement)
      (Class|AuraEffectActor|StartRotation))))

(event EventDestroyed
  (Audio|PlaySoundatLocation (Variables|Default|GetConsumedSound) (Transformation|GetActorLocation) "0, 0, 0" 1.0 1.0 0.0 0 0 0 0))

(event EventTick
  (params (DeltaSeconds :type Float%20%28single-precision%29))
  (Transformation|SetActorLocation (Variables|Default|GetCalculatedLocation) false false)
  (Transformation|SetActorRotation (Variables|Default|GetCalculatedRotation)))

(fn ConstructionScript)

(fn SetCalculatedLocation
  (params (A :type Float%20%28double-precision%29))
  (bind _initiallocation (Variables|Default|GetInitialLocation))
  (bind (_x _y _z) (Math|Vector|BreakVector _initiallocation))
  (Variables|Default|SetCalculatedLocation (Math|Vector|MakeVector _x _y (+ _z (* A (Variables|Default|GetSpawnApex))))))