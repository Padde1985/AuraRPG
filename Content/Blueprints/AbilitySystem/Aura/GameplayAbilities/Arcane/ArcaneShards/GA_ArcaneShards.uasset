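; Arcane Shards gameplay ability that shows a magic circle, then casts a series of damaging shards where the player clicks.
; A press spawns a point collection at the cursor hit for randomly rotated ground points and plays the cast montage.
; The montage event commits cost and starts a looping timer that damages live players around each point and fires a GameplayCue.
; Shard count scales with ability level up to a cap, and cooldown commits after the last shard.
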(event Custom|SpawnShard
  (if (< (Variables|Default|GetCount) (Variables|Default|GetNumShards))
    (CallFunction|StoreSpawnShardLocationandRotation)
    (CallFunction|StoreOverlappingPlayers)
    (for _array_element (Variables|Default|GetPlayersToDamage)
      (CallFunction|CauseDamagetoActor _array_element))
    (Math|Integer|IncrementInt (Variables|Default|GetCount)
      (:%20%20
        (CallFunction|ExecuteGameplayCue)))
    (else
      (Utilities|Time|ClearandInvalidateTimerbyHandle (Variables|Default|GetShardSpawnTimer))
      (Actor|DestroyActor (Variables|Default|GetPointCollection))
      (Ability|CommitAbilityCooldown false)
      (Ability|EndAbility))))

(event Ability|EventActivateAbility
  (bind _returnvalue (Class|GameplayAbility|CheckAbilityCost))
  (if _returnvalue
    (Utilities|FlowControl|Sequence
      (:then_0
        (Class|PlayerInterface|ShowMagicCircle(Message) (Ability|GetAvatarActorfromActorInfo) 0))
      (:then_1
        (Ability|Tasks|WaitInputPress false
          (:OnPress
            (bind _datahandle (|TargetDataUnderMouse)
              (:ValidData
                (CallFunction|StoreMouseHitLocation _datahandle)
                (bind _returnvalue_2 (Game|SpawnActorfromClass "/Game/Blueprints/AbilitySystem/Aura/GameplayAbilities/Arcane/ArcaneShards/BP_PointCollection.BP_PointCollection_C" (Math|Transform|MakeTransform (Variables|Default|GetMouseHitLocation) "0, 0, 0" "1.000000,1.000000,1.000000") "AlwaysSpawn" "MultiplyWithRoot" 0 0))
                (CallFunction|SetGroundPoints _returnvalue_2)
                (Class|CombatInterface|UpdateWarpTarget(Message) (Ability|GetAvatarActorfromActorInfo) (Variables|Default|GetMouseHitLocation))
                (|PlayMontageandWaitProxy "None" "/Game/Assets/Characters/Aura/Animations/Abilities/AM_Cast_ArcaneShards_Montage.AM_Cast_ArcaneShards_Montage" 1.0 "None" false 1.0 0.0 false))))))
      (:then_2
        (Ability|Tasks|WaitGameplayEvent "(TagName=\"Event.Montage.ArcaneShards\")" 0 true
          (:EventReceived
            (bind _returnvalue_3 (Utilities|Time|SetTimerbyEvent (delegate Custom|SpawnShard) (Variables|Default|GetShardSpawnDeltaTime) true))
            (Variables|Default|SetShardSpawnTimer _returnvalue_3)
            (Class|PlayerInterface|HideMagicCircle(Message) (Ability|GetAvatarActorfromActorInfo))
            (CallFunction|SpawnShard)
            (Ability|CommitAbilityCost false)))))))

(fn StoreSpawnShardLocationandRotation
  (bind _groundpoints (Variables|Default|GetGroundPoints))
  (bind _count (Variables|Default|GetCount))
  (bind _output (Utilities|Array|Get(acopy) _groundpoints _count))
  (Variables|Default|SetShardSpawnLocation (Transformation|GetWorldLocation _output))
  (Variables|Default|SetShardSpawnRotation (Transformation|GetWorldRotation _output))
  (return))

(fn StoreOverlappingPlayers
  (bind _returnvalue (Ability|GetAvatarActorfromActorInfo))
  (bind _outoverlappingactors (Class|AuraAbilitysystemLibrary|GetLivePlayersWithinRadius _returnvalue (Utilities|Array|MakeArray _returnvalue) (Variables|Default|GetRadialDamageOuterRadius) (Variables|Default|GetShardSpawnLocation)))
  (Variables|Default|SetPlayersToDamage _outoverlappingactors)
  (return))

(fn CauseDamagetoActor
  (params (TargetActor :type Actor%20Object%20Reference))
  (Class|AuraAbilitysystemLibrary|ApplyDamageEffect (Class|AuraDamageGameplayAbility|MakeDamageEffectParamsfromClassDefaults TargetActor (Variables|Default|GetShardSpawnLocation))))

(fn SetGroundPoints
  (params (PointCollection :type BP%20Point%20Collection%20Object%20Reference))
  (bind _output_get (Variables|Default|SetPointCollection PointCollection))
  (Variables|Default|SetNumShards (Math|Integer|Min(Integer) (Variables|Default|GetMaxNumShards) (Ability|GetAbilityLevel)))
  (Variables|Default|SetGroundPoints (Class|PointCollection|GetGroundPoints _output_get (Variables|Default|GetMouseHitLocation) 0 (Math|Random|RandomFloatinRange 0.0 3.6e+02))))

(fn StoreMouseHitLocation
  (params (HitResult :type Gameplay%20Ability%20Target%20Data%20Handle%20Structure%20%28by%20ref%29))
  (Variables|Default|SetMouseHitLocation (.ImpactPoint (Collision|BreakHitResult (Ability|TargetData|GetHitResultfromTargetData HitResult)))))

(fn ExecuteGameplayCue
  (Class|GameplayAbility|ExecuteGameplayCuewithParams "(TagName=\"GameplayCue.ArcaneShards\")" (Ability|GameplayCue|MakeGameplayCueParameters :Location (Variables|Default|GetShardSpawnLocation) :Normal (Math|Vector|GetRightVector (Variables|Default|GetShardSpawnRotation)))))