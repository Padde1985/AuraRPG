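; Fire Blast fireball actor that flies out to an apex, returns to its instigator and explodes on getting close.
; Server-run outgoing and returning timelines lerp its location, with the return tracking the instigator's current position.
; The explosion gathers live players in radius, excluding the owner, and applies radial damage with upward-angled knockback and death impulse through ability system damage params, then destroys the actor.
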(event EventStartOutgoingTimeline
  (Networking|SwitchHasAuthority
    (:Authority
      (Variables|Default|SetInitialLocation (Transformation|GetActorLocation))
      (CallFunction|SetApexLocation)
      (bind _outgoingtrack (Timeline|OutgoingTimeline Play)
        (:Update
          (CallFunction|UpdateOutgoingLocation _outgoingtrack))
        (:Finished
          (bind _returningtrack (Timeline|ReturningTimeline Play)
            (:Update
              (CallFunction|UpdateReturningLocation _returningtrack)
              (if (CallFunction|IsWithinExplodeDistance)
                (Class|AuraProjectile|OnHit)
                (bind _outoverlappingactors (CallFunction|SetOverlappingActors))
                (Variables|Default|SetOverlappingActors _outoverlappingactors)
                (Class|AuraAbilitysystemLibrary|SetIsRadialDamageEffectParam (Variables|Default|GetExplosionDamageParams) true (Variables|Default|GetInner%20Radius) (Variables|Default|GetOuter%20Radius) (Transformation|GetActorLocation))
                (for _array_element (Variables|Default|GetOverlappingActors)
                  (Class|AuraAbilitysystemLibrary|SetTargetEffectParamsASC (Variables|Default|GetExplosionDamageParams) (Ability|GetAbilitySystemComponent _array_element))
                  (bind _returnvalue (CallFunction|SetKnockbackDirection _array_element))
                  (Variables|Default|SetKnockbackDirection _returnvalue)
                  (Class|AuraAbilitysystemLibrary|SetKnockbackDirection (Variables|Default|GetExplosionDamageParams) (Variables|Default|GetKnockbackDirection) (Variables|Default|GetKnockbackMagnitude))
                  (Class|AuraAbilitysystemLibrary|SetDeathImpulseDirection (Variables|Default|GetExplosionDamageParams) (Variables|Default|GetKnockbackDirection) (Variables|Default|GetDeathImpulseMagnitude))
                  (Class|AuraAbilitysystemLibrary|ApplyDamageEffect (Variables|Default|GetExplosionDamageParams)))
                (Actor|DestroyActor)))))))))

(fn ConstructionScript)

(fn SetApexLocation
  (Variables|Default|SetApexLocation (+ (Variables|Default|GetInitialLocation) (* (Transformation|GetActorForwardVector) (Variables|Default|GetTravelDistance)))))

(fn UpdateOutgoingLocation
  (params (Alpha :type Float%20%28single-precision%29))
  (Transformation|SetActorLocation (Math|Vector|Lerp(Vector) (Variables|Default|GetInitialLocation) (Variables|Default|GetApexLocation) Alpha) false false))

(fn UpdateReturningLocation
  (params (Alpha :type Float%20%28single-precision%29))
  (Transformation|SetActorLocation (Math|Vector|Lerp(Vector) (Variables|Default|GetApexLocation) (Transformation|GetActorLocation (Game|GetInstigator)) Alpha) false false))

(fn IsWithinExplodeDistance
  (return (<= (Math|Vector|VectorLength (- (Transformation|GetActorLocation) (Transformation|GetActorLocation (Game|GetInstigator)))) (Variables|Default|GetExplodeDistance))))

(fn SetKnockbackDirection
  (params (self2 :type Actor%20Object%20Reference))
  (bind _returnvalue (Transformation|GetActorLocation))
  (bind _returnvalue_2 (Transformation|GetActorLocation self2))
  (bind _returnvalue_3 (- _returnvalue_2 _returnvalue))
  (bind _returnvalue_4 (Math|Rotator|MakeRotfromX _returnvalue_3))
  (return (Math|Vector|GetForwardVector (Math|Rotator|MakeRotator (.roll _returnvalue_4) 45.0 (.yaw _returnvalue_4)))))

(fn SetOverlappingActors
  (bind _outoverlappingactors (Class|AuraAbilitysystemLibrary|GetLivePlayersWithinRadius self (Utilities|Array|MakeArray (Components|GetOwner) self) (Variables|Default|GetPlayerRadius) (Transformation|GetActorLocation)))
  (return _outoverlappingactors))